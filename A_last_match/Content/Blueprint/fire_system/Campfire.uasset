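; Campfire actor whose fire burns down over time.
; A looping timer started on BeginPlay lowers the fire level at a fixed interval, clamped between zero and a maximum, and prints it on screen.
; Each tick of the timer scales the Fire component to the current level and switches the Box collision off when the fire is out, on otherwise.
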(event `self.ReceiveBeginPlay`
  (`KismetSystemLibrary.K2_SetTimerDelegate` (delegate `Firerefresh`) 2.0 true))

(event `Firerefresh`
  (set `self.firelevel` (`KismetMathLibrary.FClamp` (- (`self.firelevel`) 1.0) 0.0 (`self.Maxfirelevel`)))
  (`KismetSystemLibrary.PrintString` (`KismetStringLibrary.Conv_DoubleToString` (`self.firelevel`)) true true (struct :`R` 1.0 :`G` 0.183826 :`A` 1.0))
  (`SceneComponent.SetRelativeScale3D` (`self.fire`) (`KismetMathLibrary.Conv_DoubleToVector` (/ (`self.firelevel`) 100.0)))
  (if (<= (`self.firelevel`) 0.0)
    (`PrimitiveComponent.SetCollisionEnabled` (`self.Box`) "NoCollision")
    (else
      (`PrimitiveComponent.SetCollisionEnabled` (`self.Box`) "QueryAndPhysics"))))

(fn `UserConstructionScript`)